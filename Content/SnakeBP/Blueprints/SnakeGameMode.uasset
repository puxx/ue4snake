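; Game mode for a grid-based Snake game that spawns worms, handles self-collision death, and restarts or quits the game.
; A looping timer spawns a worm at a random grid cell when none exists, though the overlap test rolls different cells from the spawn.
; Self-collision marks the pawn dead once until ReloadGame respawns it at the camera and repossesses it.
; VectorPortal wraps out-of-bounds positions to the opposite field edge.
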(event Custom|Snake%20collision
  (Utilities|FlowControl|DoOnce false
    (:Completed
      (Development|PrintString "Eat your self!!!! BOOOO!")
      (Variables|/Game/SnakeBP/Blueprints/SnakePawn.SnakePawn_C|SetDeath (Variables|Default|GetSnakePawn) true))))

(event Custom|CreateWarmEvent
  ;[1 1 1] Spawn worm
  (CallFunction|CreateWorm))

(event Custom|Close%20game
  (Game|QuitGame (Game|GetPlayerController 0) "Quit"))

(event Custom|ReloadGame
  (bind _returnvalue (Game|GetPlayerController 0))
  (bind _returnvalue_2 (Game|GetPlayerCameraManager 0))
  (Pawn|UnPossess _returnvalue)
  (Actor|DestroyActor (Variables|Default|GetSnakePawn))
  (bind _returnvalue_3 (Game|SpawnActorfromClass "/Game/SnakeBP/Blueprints/SnakePawn.SnakePawn_C" (Math|Transform|MakeTransform (Camera|GetCameraLocation _returnvalue_2) (Camera|GetCameraRotation _returnvalue_2) "1.000000,1,1") false 0))
  (Pawn|Possess _returnvalue _returnvalue_3)
  (bind _assnake_pawn (CallFunction|GetCurrentSnakePawn))
  (Variables|Default|SetSnakePawn _assnake_pawn)
  (Utilities|FlowControl|DoOnce false) ; enters at Reset
)

(event EventBeginPlay
  (Utilities|FlowControl|Sequence
    (:then_0
      (bind _assnake_pawn (CallFunction|GetCurrentSnakePawn))
      (Variables|Default|SetSnakePawn _assnake_pawn))
    (:then_1
      (Utilities|Time|SetTimerbyEvent (delegate Custom|CreateWarmEvent) (Variables|Dificulty|GetNewWormSpawnTimeOut) true))))

(fn ConstructionScript)

(fn CreateWorm
  (bind _randomstream (Variables|Default|GetRandomStream))
  (bind _boxside (Variables|Default|GetBoxSide))
  (bind _boxside_2 (Variables|Default|GetBoxSide))
  (bind _sidea (Variables|Default|GetSideA))
  (bind _boxside_3 (Variables|Default|GetBoxSide))
  (bind _sideb (Variables|Default|GetSideB))
  (bind _boxside_4 (Variables|Default|GetBoxSide))
  (bind _boxside_5 (Variables|Default|GetBoxSide))
  (bind _returnvalue (/ _sideb _boxside_2))
  (bind _returnvalue_2 (/ _sidea _boxside_3))
  (bind _returnvalue_3 (Math|Float|Floor _returnvalue))
  (bind _returnvalue_4 (* -1 _returnvalue))
  (bind _returnvalue_5 (Math|Float|Floor _returnvalue_2))
  (bind _returnvalue_6 (* -1 _returnvalue_2))
  (bind _returnvalue_7 (Math|Float|Floor _returnvalue_4))
  (bind _returnvalue_8 (Math|Float|Floor _returnvalue_6))
  (bind _returnvalue_9 (Math|Random|RandomIntegerinRangefromStream _returnvalue_8 _returnvalue_5 _randomstream))
  (bind _returnvalue_10 (Math|Random|RandomIntegerinRangefromStream _returnvalue_7 _returnvalue_3 _randomstream))
  (bind _returnvalue_11 (* _returnvalue_9 _boxside_5))
  (bind _returnvalue_12 (* _returnvalue_10 _boxside_4))
  (bind _returnvalue_13 (Math|Vector|MakeVector _returnvalue_11 _returnvalue_12 _boxside))
  (bind _outactors (Actor|GetAllActorsOfClass "/Game/SnakeBP/Blueprints/WormActor.WormActor_C"))
  (if (not (> (Utilities|Array|Length _outactors) 0))
    (LocalVariables|SetCollisionWorm true)
    (bind _outactors_2 (Actor|GetAllActorsOfClass "/Game/SnakeBP/Blueprints/SnakePartActor.SnakePartActor_C"))
    (for _array_element _outactors_2
      (bind _output_get (LocalVariables|SetCollisionWorm (and (Math|Vector|NotEqual(Vector) _returnvalue_13 (Transformation|GetActorLocation _array_element) 0.0001) (LocalVariables|GetCollisionWorm)))))
    (if _output_get
      (Game|SpawnActorfromClass "/Game/SnakeBP/Blueprints/WormActor.WormActor_C" (Math|Transform|MakeTransform _returnvalue_13 "0.000000,0.000000,0.000000") false 0)
      (Development|PrintString "Create new sworm"))))

(fn VectorPortal
  (params (Vector :type Vector :default "0, 0, 0"))
  (bind (_x _y _z) (Math|Vector|BreakVector Vector))
  (bind _returnvalue (Math|Float|Absolute(Float) _x))
  (bind _returnvalue_2 (Math|Float|Absolute(Float) _y))
  (if (<= _returnvalue (Variables|Default|GetSideA))
    (LocalVariables|Setx_fix _x)
    (else
      (LocalVariables|Setx_fix (* (* -1 (/ _returnvalue _x)) (Variables|Default|GetSideA)))))
  (if (<= _returnvalue_2 (Variables|Default|GetSideB))
    (LocalVariables|Sety_fix _y)
    (else
      (LocalVariables|Sety_fix (* (* -1 (/ _returnvalue_2 _y)) (Variables|Default|GetSideB)))))
  (return (Math|Vector|MakeVector (LocalVariables|Getx_fix) (LocalVariables|Gety_fix) _z)))

(fn GetCurrentSnakePawn
  (bind _assnake_pawn (Utilities|Casting|CastToSnakePawn (Game|Player|GetPlayerPawn 0))
    (:then
      (return _assnake_pawn))
    (:CastFailed
      (Development|PrintString "fail to"))))