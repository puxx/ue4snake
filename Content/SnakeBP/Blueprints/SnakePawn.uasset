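; Player snake pawn for a Snake game, built from spawned SnakePartActor boxes.
; Tick throttles movement by Snake.Speed, then advances using a ring buffer: one part teleports one box ahead of the head, through GameMode.VectorPortal.
; EatWorm destroys the worm, inserts a new part and raises speed by the GameMode increment.
; On Death, movement stops and a timeline blinks the body; destroying the pawn destroys its parts.
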(event Custom|EatWorm
  (params (Worm :type Worm%20Actor%20Object%20Reference%20%28by%20ref%29))
  (bind _snake (Variables|Default|GetSnake))
  (bind _snake_2 (Variables|Default|GetSnake))
  (bind (_currentdirection _newdiewction _speed _lenght _snakemass) (Utilities|Struct|Breaksnakestruct _snake))
  (bind (_currentdirection_2 _newdiewction_2 _speed_2 _lenght_2 _snakemass_2) (Utilities|Struct|Breaksnakestruct _snake_2))
  ;[1 1 1] Eat worm event
  (Actor|DestroyActor Worm)
  (bind _output_get (Variables|Default|Setworm_counter (+ (Variables|Default|Getworm_counter) 1)))
  (bind _newsnakepart (CallFunction|CreateNewSnakePart _output_get))
  (Utilities|Array|Insert _snakemass _newsnakepart _lenght)
  (Utilities|Struct|Setmembersinsnakestruct _snake_2 (+ (Variables|/Game/SnakeBP/Blueprints/SnakeGameMode.SnakeGameMode_C|GetSpeedInc (Variables|Default|GetGameMode)) _speed_2) (Utilities|Array|Length _snakemass_2)))

(event EventBeginPlay
  (bind _snake (Variables|Default|GetSnake))
  (bind (_currentdirection _newdiewction _speed _lenght _snakemass) (Utilities|Struct|Breaksnakestruct _snake))
  ;[1 1 1] Create snake
  (bind (_currentindex _lastindex) (CallFunction|InitSnake _snakemass _lenght (Variables|Default|GetStartPoint) (Variables|Default|Getbox_side)))
  (Variables|MoveSnake|Setcurrent_index _currentindex)
  (Variables|MoveSnake|Setlast_index _lastindex))

(event EventTick
  (params (DeltaSeconds :type Float%20%28single-precision%29))
  (bind _snake (Variables|Default|GetSnake))
  (bind (_currentdirection _newdiewction _speed _lenght _snakemass) (Utilities|Struct|Breaksnakestruct _snake))
  (if (Variables|Default|GetDeath)
    ;[1 1 1] Blink on death
    (Utilities|FlowControl|DoOnce false
      (:Completed
        (bind _blinkfreq (Timeline|BlinkTimeline Play)
          (:Update
            (for _array_element (.snakeMass (Utilities|Struct|Breaksnakestruct (Variables|Default|GetSnake)))
              (Rendering|SetActorHiddenInGame _array_element (> _blinkfreq 0.0)))))))
    (else
      ;[1 1 1] MoveSnake
      (Utilities|SpeedControl DeltaSeconds _speed)
      (CallFunction|MoveSnake _currentdirection _snakemass))))

(event EventDestroyed
  (for _array_element (.snakeMass (Utilities|Struct|Breaksnakestruct (Variables|Default|GetSnake)))
    (Actor|DestroyActor _array_element)))

(fn ConstructionScript
  (bind _snake (Variables|Default|GetSnake))
  (bind (_currentdirection _newdiewction _speed _lenght _snakemass) (Utilities|Struct|Breaksnakestruct _snake))
  (bind _assnake_game_mode (Utilities|Casting|CastToSnakeGameMode (Game|GetGameMode)))
  (bind _output_get (Variables|Default|SetGameMode _assnake_game_mode))
  (Variables|Default|Setbox_side (Variables|/Game/SnakeBP/Blueprints/SnakeGameMode.SnakeGameMode_C|GetBoxSide _output_get))
  (while (< (Utilities|Array|Length _snakemass) _lenght)
    (Utilities|Array|Insert _snakemass (stale _assnake_part_actor))))

(fn InitSnake
  (params (Mass :type Array%20of%20Snake%20Part%20Actor%20Object%20References) (Lenght :type Integer :default 0) (StartPoint :type Vector%202D%20Structure) (BoxSide :type Float%20%28single-precision%29 :default 0.0))
  (bind (_x _y) (Math|Vector2D|BreakVector2D StartPoint))
  (for (_ _array_index) Mass
    (bind _returnvalue (Game|SpawnActorfromClass "/Game/SnakeBP/Blueprints/SnakePartActor.SnakePartActor_C" (Math|Transform|MakeTransform (Math|Conversions|ToVector(Vector2D) (Math|Vector2D|MakeVector2D (+ _x (* (+ _array_index 1) BoxSide)) _y) BoxSide) "0, 0,0.000000") false 0))
    (Variables|/Game/SnakeBP/Blueprints/SnakePartActor.SnakePartActor_C|SetSnakePawn _returnvalue self)
    (Utilities|Array|SetArrayElem Mass _array_index _returnvalue))
  (bind _output_get (LocalVariables|Setcurrent_index (- Lenght 1)))
  (LocalVariables|Setlast_index (- _output_get 1))
  (return (LocalVariables|Getcurrent_index) (LocalVariables|Getlast_index)))

(fn MoveSnake
  (params (Direction :type snakestates%20Enum :default "NewEnumerator0") (Array :type Array%20of%20Snake%20Part%20Actor%20Object%20References))
  (bind _snake (Variables|Default|GetSnake))
  (bind _newdiewction (Utilities|Struct|Breaksnakestruct _snake))
  (Utilities|FlowControl|Sequence
    (:then_0
      (switch Utilities|FlowControl|Switch|Switchonsnakestates Direction
        (:NewEnumerator0
          (Variables|MoveSnake|Setx_shift (Variables|Default|Getbox_side))
          (Variables|MoveSnake|Sety_shift 0.0))
        (:NewEnumerator1
          (Variables|MoveSnake|Setx_shift (* -1 (Variables|Default|Getbox_side)))
          (Variables|MoveSnake|Sety_shift 0.0))
        (:NewEnumerator2
          (Variables|MoveSnake|Setx_shift 0.0)
          (Variables|MoveSnake|Sety_shift (Variables|Default|Getbox_side)))
        (:NewEnumerator3
          (Variables|MoveSnake|Setx_shift 0.0)
          (Variables|MoveSnake|Sety_shift (* -1 (Variables|Default|Getbox_side))))))
    (:then_1
      (Rendering|SetActorHiddenInGame (Utilities|Array|Get(acopy) Array (Variables|MoveSnake|Getcurrent_index)) true)
      (bind _result (Default|VectorPortal (Variables|Default|GetGameMode) (+ (Transformation|GetActorLocation (Utilities|Array|Get(acopy) Array (Variables|MoveSnake|Getlast_index))) (Math|Vector|MakeVector (Variables|MoveSnake|Getx_shift) (Variables|MoveSnake|Gety_shift) 0.0))))
      (Transformation|Teleport (Utilities|Array|Get(acopy) Array (Variables|MoveSnake|Getcurrent_index)) _result "0, 0, 0")
      (Rendering|SetActorHiddenInGame (Utilities|Array|Get(acopy) Array (Variables|MoveSnake|Getcurrent_index)) false)
      ;[1 1 1] Update snake current direction
      (Utilities|Struct|Setmembersinsnakestruct _snake _newdiewction _newdiewction))
    (:then_2
      ;[1 1 1] Upfate index
      (Variables|MoveSnake|Setlast_index (Variables|MoveSnake|Getcurrent_index))
      (Variables|MoveSnake|Setcurrent_index (+ 1 (Variables|MoveSnake|Getcurrent_index)))
      (if (== (Variables|MoveSnake|Getcurrent_index) (Utilities|Array|Length Array))
        (Variables|MoveSnake|Setcurrent_index 0)))))

(fn CreateNewSnakePart
  (params (Poistion :type Integer))
  (bind _returnvalue (Game|SpawnActorfromClass "/Game/SnakeBP/Blueprints/SnakePartActor.SnakePartActor_C" (Math|Transform|MakeTransform (Math|Vector|MakeVector 1e+03 (* Poistion (Variables|Default|Getbox_side)) 0.0) "0, 0,0.000000") false 0))
  (Variables|/Game/SnakeBP/Blueprints/SnakePartActor.SnakePartActor_C|SetSnakePawn _returnvalue self)
  (return _returnvalue))