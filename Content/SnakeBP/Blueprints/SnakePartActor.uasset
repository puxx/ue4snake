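; SnakePartActor is a single segment of the player's snake that detects what it overlaps.
; On BeginPlay it caches the SnakeGameMode and the player's SnakePawn.
; Overlapping another snake part reports a self-collision to the game mode and prints the location, while overlapping a WormActor tells the pawn to eat that worm.
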(event EventBeginPlay
  (bind _assnake_game_mode (Utilities|Casting|CastToSnakeGameMode (Game|GetGameMode)))
  (Variables|Default|SetGameMode _assnake_game_mode)
  (bind _assnake_pawn (Utilities|Casting|CastToSnakePawn (Game|Player|GetPlayerPawn 0)))
  (Variables|Default|SetSnakePawn _assnake_pawn))

(event EventActorBeginOverlap
  (params (OtherActor :type Actor%20Object%20Reference))
  (bind _assnake_part_actor (Utilities|Casting|CastToSnakePartActor OtherActor)
    (:then
      (Default|SnakeCollision (Variables|Default|GetGameMode))
      (Development|PrintString (Utilities|String|BuildString(Vector) "" "Collision location:" (Transformation|GetActorLocation _assnake_part_actor))))
    (:CastFailed
      (bind _asworm_actor (Utilities|Casting|CastToWormActor OtherActor)
        (:then
          (Default|EatWorm (Variables|Default|GetSnakePawn) _asworm_actor))
        (:CastFailed
          (Development|PrintString "Cast failed"))))))

(event EventTick
  (params (DeltaSeconds :type Float%20%28single-precision%29)))

(fn ConstructionScript)