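; Player controller for a Snake game that handles steering, pause, reload and quit input.
; Move axes set the SnakePawn's new direction in its Snake struct, only when the current direction is on the other axis, preventing reversals.
; Pause toggles game pause through a FlipFlop with on-screen messages.
; Jump and Escape call reload and close on the SnakeGameMode, cached in the Construction Script.
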(event EventBeginPlay)

(event Input|ActionEvents|InputActionJump
  (:Pressed
    (Default|ReloadGame (Variables|Default|GetGameMode))))

(event Input|ActionEvents|InputActionPause
  ;[1 1 1] Pause
  (:Pressed
    (Utilities|FlowControl|FlipFlop
      (:A
        (Game|SetGamePaused true)
        (Development|PrintString "Paused!"))
      (:B
        (Game|SetGamePaused false)
        (Development|PrintString "Unpaused")))))

(event Input|KeyboardEvents|Escape
  (:Pressed
    (Default|CloseGame (Variables|Default|GetGameMode))))

(event Input|AxisEvents|InputAxisMoveForward
  (params (AxisValue :type Float%20%28single-precision%29))
  (Utilities|FlowControl|Sequence
    (:then_0
      ;[1 1 1] Snake move controller
      (bind _assnake_pawn (Utilities|Casting|CastToSnakePawn (Game|Player|GetPlayerPawn 0))))
    (:then_1
      (Math|Float|CompareFloat AxisValue 0.0
        (:>
          (Variables|MoveSnake|Setinput_state "NewEnumerator0"))
        (:<
          (Variables|MoveSnake|Setinput_state "NewEnumerator1")))
      (if (or (Utilities|Enum|Equal(Enum) (.CurrentDirection (Utilities|Struct|Breaksnakestruct (Variables|/Game/SnakeBP/Blueprints/SnakePawn.SnakePawn_C|GetSnake _assnake_pawn))) "NewEnumerator2") (Utilities|Enum|Equal(Enum) (.CurrentDirection (Utilities|Struct|Breaksnakestruct (Variables|/Game/SnakeBP/Blueprints/SnakePawn.SnakePawn_C|GetSnake _assnake_pawn))) "NewEnumerator3"))
        (Utilities|Struct|Setmembersinsnakestruct (Variables|/Game/SnakeBP/Blueprints/SnakePawn.SnakePawn_C|GetSnake _assnake_pawn) (Variables|MoveSnake|Getinput_state))))))

(event Input|AxisEvents|InputAxisMoveRight
  (params (AxisValue :type Float%20%28single-precision%29))
  (Utilities|FlowControl|Sequence
    (:then_0
      ;[1 1 1] Snake move controller
      (bind _assnake_pawn (Utilities|Casting|CastToSnakePawn (Game|Player|GetPlayerPawn 0))))
    (:then_1
      (Math|Float|CompareFloat AxisValue 0.0
        (:>
          (Variables|MoveSnake|Setinput_state "NewEnumerator3"))
        (:<
          (Variables|MoveSnake|Setinput_state "NewEnumerator2")))
      (if (or (Utilities|Enum|Equal(Enum) (.CurrentDirection (Utilities|Struct|Breaksnakestruct (Variables|/Game/SnakeBP/Blueprints/SnakePawn.SnakePawn_C|GetSnake _assnake_pawn))) "NewEnumerator0") (Utilities|Enum|Equal(Enum) (.CurrentDirection (Utilities|Struct|Breaksnakestruct (Variables|/Game/SnakeBP/Blueprints/SnakePawn.SnakePawn_C|GetSnake _assnake_pawn))) "NewEnumerator1"))
        (Utilities|Struct|Setmembersinsnakestruct (Variables|/Game/SnakeBP/Blueprints/SnakePawn.SnakePawn_C|GetSnake _assnake_pawn) (Variables|MoveSnake|Getinput_state))))))

(fn ConstructionScript
  (bind _assnake_game_mode (Utilities|Casting|CastToSnakeGameMode (Game|GetGameMode)))
  (Variables|Default|SetGameMode _assnake_game_mode))