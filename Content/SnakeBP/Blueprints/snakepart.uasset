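; Actor Blueprint for one segment of the snake, which detects self-collision and worm pickups through overlap events.
; Overlapping another snakepart calls SnakeCollision on the SnakeGameMode and prints the collision location.
; Overlapping a WormActor passes it to EatWorm on the gamer player controller.
; The Move function and construction script are empty, so the segment has no movement logic of its own.
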(event EventActorBeginOverlap
  (params (OtherActor :type Actor%20Object%20Reference))
  (bind _assnakepart (Utilities|Casting|CastTosnakepart OtherActor)
    (:then
      (bind _assnake_game_mode (Utilities|Casting|CastToSnakeGameMode (Game|GetGameMode))
        (:then
          (Default|SnakeCollision _assnake_game_mode)
          (Development|PrintString (Utilities|String|BuildString(Vector) "" "Collision location:" (Transformation|GetActorLocation _assnakepart))))
        (:CastFailed
          (Development|PrintString "Cast failed"))))
    (:CastFailed
      (bind _asworm_actor (Utilities|Casting|CastToWormActor OtherActor)
        (:then
          (bind _asgamer (Utilities|Casting|CastTogamer (Game|GetPlayerController 0)))
          (Default|EatWorm _asgamer _asworm_actor)
          (Development|PrintString "Snake eat sworm"))
        (:CastFailed
          (Development|PrintString "Cast failed"))))))

(fn ConstructionScript)

(fn Move)