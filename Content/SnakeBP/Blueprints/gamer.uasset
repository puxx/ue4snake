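; Snake game controller that builds the snake from SnakePart actors and handles input, pause, worm spawning, growth and death blinking.
; On a Tick-accumulated interval, MoveSnake teleports one segment ahead of the head using a cycling index, wrapping at field edges via VectorPortal.
; Axis input queues perpendicular turns only.
; A looping timer spawns a random worm when none exists; EatWorm adds a segment and shortens the move interval.
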(event Custom|CreateSwarm
  ;[1 1 1] Spawn worm
  (CallFunction|CreateWorm))

(event Custom|EatWorm
  (params (Worm :type Worm%20Actor%20Object%20Reference%20%28by%20ref%29))
  (bind _snake (Variables|Main|GetSnake))
  (bind _snake_2 (Variables|Main|GetSnake))
  (bind (_currentdirection _newdiewction _speed _lenght _snakemass) (Utilities|Struct|Breaksnakestruct _snake))
  (bind (_currentdirection_2 _newdiewction_2 _speed_2 _lenght_2 _snakemass_2) (Utilities|Struct|Breaksnakestruct _snake_2))
  ;[1 1 1] On eat worm event
  (Actor|DestroyActor Worm)
  (bind _output_get (Variables|Default|Setworm_counter (+ (Variables|Default|Getworm_counter) 1)))
  (bind _returnvalue (Game|SpawnActorfromClass "/Game/SnakeBP/Blueprints/SnakePartActor.SnakePartActor_C" (Math|Transform|MakeTransform (Math|Vector|MakeVector 1e+03 (* _output_get (Variables|Constants|Getbox_side)) 0.0) "0, 0,0.000000") false 0))
  (Utilities|Array|Insert _snakemass _returnvalue _lenght)
  (Utilities|Struct|Setmembersinsnakestruct _snake_2 (* _speed_2 0.9) (Utilities|Array|Length _snakemass_2) _snakemass_2)
  (Development|PrintString (Utilities|String|BuildString(Integer) "" "Current index = " (Variables|MoveSnake|Getcurrent_index)) true true "(R=1.000000,G=0.039531,B=0.068183,A=1.000000)"))

(event EventTick
  (params (DeltaSeconds :type Float%20%28single-precision%29))
  (bind _snake (Variables|Main|GetSnake))
  (bind (_currentdirection _newdiewction _speed _lenght _snakemass) (Utilities|Struct|Breaksnakestruct _snake))
  (if (Variables|Main|GetDeath)
    (Utilities|FlowControl|DoOnce false
      (:Completed
        ;[1 1 1] Blink on death
        (Utilities|FlowControl|Sequence
          (:then_0
            (bind _blinkfreq (Timeline|DeathBlink Play)
              (:Update
                (for _array_element 0
                  (Rendering|SetVisibility _array_element (> _blinkfreq 0.0) true)))))
          (:then_1
            (Development|PrintString (Utilities|String|BuildString(Integer) "" "Size:" (.lenght (Utilities|Struct|Breaksnakestruct (Variables|Main|GetSnake)))))))))
    (else
      ;[1 1 1] MoveSnake
      (if (>= (Variables|Default|Getspeed_counter) _speed)
        (Variables|Default|Setspeed_counter 0.0)
        (CallFunction|MoveSnake _currentdirection _snakemass _lenght)
        (else
          (Variables|Default|Setspeed_counter (+ (Variables|Default|Getspeed_counter) DeltaSeconds)))))))

(event EventBeginPlay
  (bind _snake (Variables|Main|GetSnake))
  (bind (_currentdirection _newdiewction _speed _lenght _snakemass) (Utilities|Struct|Breaksnakestruct _snake))
  (Utilities|FlowControl|Sequence
    (:then_0
      (CallFunction|InitSnake _snakemass _lenght))
    (:then_1
      (Utilities|Time|SetTimerbyEvent (delegate Custom|CreateSwarm) 1.0 true))))

(event Input|ActionEvents|InputActionPause
  ;[1 1 1] Pause
  (:Pressed
    (Utilities|FlowControl|FlipFlop
      (:A
        (Game|SetGamePaused true)
        (Development|PrintString "Paused!"))
      (:B
        (Game|SetGamePaused false)
        (Development|PrintString "Unpaused")))))

(event Input|AxisEvents|InputAxisMoveForward
  (params (AxisValue :type Float%20%28single-precision%29))
  (bind _snake (Variables|Main|GetSnake))
  (bind (_currentdirection _newdiewction _speed _lenght _snakemass) (Utilities|Struct|Breaksnakestruct _snake))
  ;[1 1 1] Snake move controller
  (Math|Float|CompareFloat AxisValue 0.0
    (:>
      (Variables|MoveSnake|Setinput_state "NewEnumerator0"))
    (:<
      (Variables|MoveSnake|Setinput_state "NewEnumerator1")))
  (if (or (Utilities|Enum|Equal(Enum) _currentdirection "NewEnumerator2") (Utilities|Enum|Equal(Enum) _currentdirection "NewEnumerator3"))
    (Utilities|Struct|Setmembersinsnakestruct _snake _currentdirection (Variables|MoveSnake|Getinput_state) _speed _lenght _snakemass)))

(event Input|AxisEvents|InputAxisMoveRight
  (params (AxisValue :type Float%20%28single-precision%29))
  (bind _snake (Variables|Main|GetSnake))
  (bind (_currentdirection _newdiewction _speed _lenght _snakemass) (Utilities|Struct|Breaksnakestruct _snake))
  ;[1 1 1] Snake move controller
  (Math|Float|CompareFloat AxisValue 0.0
    (:>
      (Variables|MoveSnake|Setinput_state "NewEnumerator3"))
    (:<
      (Variables|MoveSnake|Setinput_state "NewEnumerator2")))
  (if (or (Utilities|Enum|Equal(Enum) _currentdirection "NewEnumerator0") (Utilities|Enum|Equal(Enum) _currentdirection "NewEnumerator1"))
    (Utilities|Struct|Setmembersinsnakestruct _snake _currentdirection (Variables|MoveSnake|Getinput_state) _speed _lenght _snakemass)))

(fn ConstructionScript
  (CallFunction|CreateSnakeArray))

(fn MoveSnake
  (params (Direction :type snakestates%20Enum%20%28by%20ref%29) (TargetArray :type Array%20of%20Snake%20Part%20Actor%20Object%20References) (Lenght :type Integer :default 0))
  (bind _snake (Variables|Main|GetSnake))
  (bind _newdiewction (Utilities|Struct|Breaksnakestruct _snake))
  (Utilities|FlowControl|Sequence
    (:then_0
      (switch Utilities|FlowControl|Switch|Switchonsnakestates Direction
        (:NewEnumerator0
          (Variables|MoveSnake|Setx_shift (Variables|Constants|Getbox_side))
          (Variables|MoveSnake|Sety_shift 0.0))
        (:NewEnumerator1
          (Variables|MoveSnake|Setx_shift (* -1 (Variables|Constants|Getbox_side)))
          (Variables|MoveSnake|Sety_shift 0.0))
        (:NewEnumerator2
          (Variables|MoveSnake|Setx_shift 0.0)
          (Variables|MoveSnake|Sety_shift (Variables|Constants|Getbox_side)))
        (:NewEnumerator3
          (Variables|MoveSnake|Setx_shift 0.0)
          (Variables|MoveSnake|Sety_shift (* -1 (Variables|Constants|Getbox_side))))))
    (:then_1
      (bind _result (CallFunction|VectorPortal (+ (Transformation|GetActorLocation (Utilities|Array|Get(acopy) TargetArray (Variables|MoveSnake|Getlast_index))) (Math|Vector|MakeVector (Variables|MoveSnake|Getx_shift) (Variables|MoveSnake|Gety_shift) 0.0)) 7e+02 7e+02))
      (Rendering|SetActorHiddenInGame (Utilities|Array|Get(acopy) TargetArray (Variables|MoveSnake|Getcurrent_index)) true)
      (Transformation|Teleport (Utilities|Array|Get(acopy) TargetArray (Variables|MoveSnake|Getcurrent_index)) _result "0, 0, 0")
      (Rendering|SetActorHiddenInGame (Utilities|Array|Get(acopy) TargetArray (Variables|MoveSnake|Getcurrent_index)) false)
      ;[1 1 1] Update snake current direction
      (Utilities|Struct|Setmembersinsnakestruct _snake _newdiewction _newdiewction))
    (:then_2
      (Variables|MoveSnake|Setlast_index (Variables|MoveSnake|Getcurrent_index))
      (Variables|MoveSnake|Setcurrent_index (+ 1 (Variables|MoveSnake|Getcurrent_index)))
      (if (== (Variables|MoveSnake|Getcurrent_index) Lenght)
        (Variables|MoveSnake|Setcurrent_index 0)))))

(fn InitSnake
  (params (Array :type Array%20of%20Snake%20Part%20Actor%20Object%20References) (Length :type Integer%20%28by%20ref%29))
  (bind _box_side (Variables|Constants|Getbox_side))
  (bind _startpoint (Variables|Constants|GetStartPoint))
  (bind (_x _y) (Math|Vector2D|BreakVector2D _startpoint))
  (for (_ _array_index) Array
    (bind _returnvalue (Game|SpawnActorfromClass "/Game/SnakeBP/Blueprints/SnakePartActor.SnakePartActor_C" (Math|Transform|MakeTransform (Math|Conversions|ToVector(Vector2D) (Math|Vector2D|MakeVector2D (+ _x (* (+ _array_index 1) _box_side)) _y) _box_side) "0, 0,0.000000") false 0))
    (Utilities|Array|SetArrayElem Array _array_index _returnvalue))
  (bind _output_get (Variables|MoveSnake|Setcurrent_index (- Length 1)))
  (Variables|MoveSnake|Setlast_index (- _output_get 1)))

(fn VectorPortal
  (params (Vector :type Vector :default "0, 0, 0") (SideA :type Float%20%28single-precision%29 :default 0.0) (SideB :type Float%20%28single-precision%29 :default 0.0))
  (bind (_x _y _z) (Math|Vector|BreakVector Vector))
  (bind _returnvalue (Math|Float|Absolute(Float) _x))
  (bind _returnvalue_2 (Math|Float|Absolute(Float) _y))
  (if (<= _returnvalue SideA)
    (Variables|VectorPortal|Setx_fix _x)
    (else
      (Variables|VectorPortal|Setx_fix (* (* -1 (/ _returnvalue _x)) SideA))))
  (if (<= _returnvalue_2 SideB)
    (Variables|VectorPortal|Sety_fix _y)
    (else
      (Variables|VectorPortal|Sety_fix (* (* -1 (/ _returnvalue_2 _y)) SideB))))
  (return (Math|Vector|MakeVector (Variables|VectorPortal|Getx_fix) (Variables|VectorPortal|Gety_fix) _z)))

(fn CreateSnakeArray
  (bind _snake (Variables|Main|GetSnake))
  (bind (_currentdirection _newdiewction _speed _lenght _snakemass) (Utilities|Struct|Breaksnakestruct _snake))
  (while (< (Utilities|Array|Length _snakemass) _lenght)
    (Utilities|Array|Insert _snakemass (stale _assnake_part_actor))
    (return))
  (return))

(fn CreateWorm
  (bind _box_side (Variables|Constants|Getbox_side))
  (bind _random_stream (Variables|Default|Getrandom_stream))
  (bind _returnvalue (Math|Random|RandomIntegerinRangefromStream -7 7 _random_stream))
  (bind _returnvalue_2 (Math|Random|RandomIntegerinRangefromStream -7 7 _random_stream))
  (bind _returnvalue_3 (* _returnvalue 100))
  (bind _returnvalue_4 (* _returnvalue_2 100))
  (bind _returnvalue_5 (Math|Conversions|ToFloat(Integer) _returnvalue_3))
  (bind _returnvalue_6 (Math|Conversions|ToFloat(Integer) _returnvalue_4))
  (bind _returnvalue_7 (Math|Vector|MakeVector _returnvalue_5 _returnvalue_6 _box_side))
  (bind _outactors (Actor|GetAllActorsOfClass "/Game/SnakeBP/Blueprints/WormActor.WormActor_C"))
  (if (> (Utilities|Array|Length _outactors) 0)
    _
    (else
      (Variables|CreateNewWorm|SetCollisionWorm true)
      (bind _outactors_2 (Actor|GetAllActorsOfClass "/Game/SnakeBP/Blueprints/snakepart.snakepart_C"))
      (bind _output_get (Variables|CreateNewWorm|SetActors _outactors_2))
      (for _array_element _output_get
        ;[1 1 1] problem zone
        (bind _output_get_2 (Variables|CreateNewWorm|SetCollisionWorm (and (Math|Vector|NotEqual(Vector) _returnvalue_7 (Transformation|GetActorLocation _array_element) 0.0001) (Variables|CreateNewWorm|GetCollisionWorm)))))
      (if _output_get_2
        (Game|SpawnActorfromClass "/Game/SnakeBP/Blueprints/WormActor.WormActor_C" (Math|Transform|MakeTransform _returnvalue_7 "0.000000,0.000000,0.000000") false 0)
        (Development|PrintString "Create new sworm"))))
  (return))